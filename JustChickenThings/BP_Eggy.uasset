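; BP_Eggy is a player-controlled rolling physics pawn, likely an egg, with a follow camera.
; Movement axes add force to its Sphere along the camera's forward and right vectors, scaled by RollingForce.
; Mouse and gamepad axes turn the controller, with gamepad input scaled by turn rate and frame time.
; Interact sets InteractAttempt while held and calls MoveBoxMessage on the Box_BP found by class on press and release.
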(event Input|ActionEvents|InputActionInteract
  (params (Key :type Key%20Structure))
  ;[0.05098 0.05098 0.05098] Interact
  (:Pressed
    (Variables|Default|SetInteract%20Attempt true)
    (bind _returnvalue (Actor|GetActorOfClass "/Game/Blueprints/Box_BP.Box_BP_C"))
    (Class|InterfaceControl|MoveBox(Message) _returnvalue))
  (:Released
    (Variables|Default|SetInteract%20Attempt false)
    (bind _returnvalue_2 (Actor|GetActorOfClass "/Game/Blueprints/Box_BP.Box_BP_C"))
    (Class|InterfaceControl|MoveBox(Message) _returnvalue_2)))

(event Input|AxisEvents|InputAxisMoveForward/Backward
  (params (AxisValue :type Float%20%28single-precision%29))
  (Physics|AddForce (Variables|Default|GetSphere) (* (Math|Vector|GetForwardVector (Variables|Camera|GetFollowCamera)) (* AxisValue (Variables|Default|GetRolling%20Force))) "None" false))

(event Input|AxisEvents|InputAxisTurnRight/LeftGamepad
  (params (AxisValue :type Float%20%28single-precision%29))
  ;[0.05098 0.05098 0.05098] Camera Input - Gamepad
  (Pawn|Input|AddControllerYawInput (* AxisValue (Variables|Input|GetTurnRateGamepad) (Utilities|Time|GetWorldDeltaSeconds))))

(event Input|AxisEvents|InputAxisTurnRight/LeftMouse
  (params (AxisValue :type Float%20%28single-precision%29))
  ;[0.05098 0.05098 0.05098] Camera Input - Mouse
  (Pawn|Input|AddControllerYawInput AxisValue))

(event Input|AxisEvents|InputAxisLookUp/DownMouse
  (params (AxisValue :type Float%20%28single-precision%29))
  ;[0.05098 0.05098 0.05098] Camera Input - Mouse
  (Pawn|Input|AddControllerPitchInput AxisValue))

(event Input|AxisEvents|InputAxisLookUp/DownGamepad
  (params (AxisValue :type Float%20%28single-precision%29))
  ;[0.05098 0.05098 0.05098] Camera Input - Gamepad
  (Pawn|Input|AddControllerPitchInput (* AxisValue (Variables|Input|GetTurnRateGamepad) (Utilities|Time|GetWorldDeltaSeconds))))

(event Input|AxisEvents|InputAxisMoveRight/Left
  (params (AxisValue :type Float%20%28single-precision%29))
  (Physics|AddForce (Variables|Default|GetSphere) (* (Math|Vector|GetRightVector (Variables|Camera|GetFollowCamera)) (* AxisValue (Variables|Default|GetRolling%20Force))) "None" false))

(fn ConstructionScript)