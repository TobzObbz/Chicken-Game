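; A pushable box Blueprint that the player character can carry while attempting to interact.
; Pawn overlaps on its Box trigger set a collision flag and check the character's InteractAttempt, so carrying only starts if interact is active on overlap begin.
; A fast looping timer then snaps the Cube to the character's GrabLocation until InteractAttempt drops, which clears the timer.
; It moves without sweep or physics; the PhysicsHandle is unused.
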(event OnComponentBeginOverlap(Box)
  (params (OverlappedComponent :type Primitive%20Component%20Object%20Reference) (OtherActor :type Actor%20Object%20Reference) (OtherComp :type Primitive%20Component%20Object%20Reference) (OtherBodyIndex :type Integer) (bFromSweep :type Boolean) (SweepResult :type Hit%20Result%20Structure%20%28by%20ref%29))
  (Utilities|Casting|CastToPawn OtherActor)
  (Variables|Default|SetInCollision? true)
  (CallFunction|MoveBox))

(event OnComponentEndOverlap(Box)
  (params (OverlappedComponent :type Primitive%20Component%20Object%20Reference) (OtherActor :type Actor%20Object%20Reference) (OtherComp :type Primitive%20Component%20Object%20Reference) (OtherBodyIndex :type Integer))
  (Utilities|Casting|CastToPawn OtherActor)
  (Variables|Default|SetInCollision? false)
  (CallFunction|MoveBox))

(event Custom|BoxMove
  (bind _asbp_third_person_character (Utilities|Casting|CastToBP_ThirdPersonCharacter (Game|GetPlayerCharacter 0)))
  (if (Variables|/Game/ThirdPerson/Blueprints/BP_ThirdPersonCharacter.BP_ThirdPersonCharacter_C|GetInteract%20Attempt _asbp_third_person_character)
    (Transformation|SetWorldLocation (Variables|Default|GetCube) (Transformation|GetWorldLocation (Variables|/Game/ThirdPerson/Blueprints/BP_ThirdPersonCharacter.BP_ThirdPersonCharacter_C|GetGrabLocation _asbp_third_person_character)) false false)
    (else
      (Utilities|Time|ClearandInvalidateTimerbyHandle (Variables|Default|GetTimer%20Handle)))))

(event EventMoveBox
  (bind _asbp_third_person_character (Utilities|Casting|CastToBP_ThirdPersonCharacter (Game|GetPlayerCharacter 0)))
  (if (and (Variables|/Game/ThirdPerson/Blueprints/BP_ThirdPersonCharacter.BP_ThirdPersonCharacter_C|GetInteract%20Attempt _asbp_third_person_character) (Variables|Default|GetInCollision?))
    (bind _returnvalue (Utilities|Time|SetTimerbyEvent (delegate Custom|BoxMove) 0.01 true))
    (Variables|Default|SetTimer%20Handle _returnvalue)))

(fn ConstructionScript)